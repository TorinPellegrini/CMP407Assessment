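; BP_CrystalSoundManager is an actor that keeps the crystal sound nearest the player prominent while ducking the rest.
; Each Tick it loops over the CrystalSounds array to find the one closest to the player pawn cached at BeginPlay.
; It sends an Attack trigger to that crystal's MetaSound and Release to all others, fading volume between full and low.
; A distance-based pause pass is left unconnected because it did not work correctly.
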(event EventBeginPlay
  (Variables|Default|SetPlayerReference (Game|Player|GetPlayerPawn 0)))

(event Collision|EventActorBeginOverlap
  (params (OtherActor :type Actor%20Object%20Reference)))

(event EventTick
  (params (DeltaSeconds :type Float%20%28single-precision%29))
  ;[1 1 1] Always reset the closest distance.
  (Variables|Default|SetClosestDistance 999999999.0)
  (for _array_element (Variables|Default|GetCrystalSounds)
    ;[0.7 0.644 1] Find the closest sound to the player.
    (if (< (Math|Vector|Distance(Vector) (Transformation|GetActorLocation _array_element) (Transformation|GetActorLocation (Variables|Default|GetPlayerReference))) (Variables|Default|GetClosestDistance))
      (Variables|Default|SetClosestAudio _array_element)
      (Variables|Default|SetClosestDistance (Math|Vector|Distance(Vector) (Transformation|GetActorLocation _array_element) (Transformation|GetActorLocation (Variables|Default|GetPlayerReference))))))
  ;[0.9812 1 0.3615] Fade in (Execute an attack) the closest sound so that it is at 100% volume, for all other sounds fade out (execute a release) until they are at 10% volume.
  (Class|AudioParameterControllerInterface|SetTriggerParameter(Message) (Variables|/Script/Engine.AmbientSound|GetAudioComponent (Variables|Default|GetClosestAudio)) "Attack")
  (for _array_element_2 (Variables|Default|GetCrystalSounds)
    (if (!= _array_element_2 (Variables|Default|GetClosestAudio))
      (Class|AudioParameterControllerInterface|SetTriggerParameter(Message) (Variables|/Script/Engine.AmbientSound|GetAudioComponent _array_element_2) "Release"))))

(fn ConstructionScript)
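; BP_DialogueBubble is a proximity audio actor that brings dialogue forward when something overlaps its configurable-radius sphere.
; Audio starts at low volume; entering raises it and pushes the SC_DialogueMix sound mix, while leaving pops the mix and lowers it.
; When IsPlayerSound is set, audio starts paused, then unpauses on overlap and calls Play only the first time.
; Overlaps are not filtered by actor.
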(event OnComponentBeginOverlap(Sphere)
  (params (OverlappedComponent :type Primitive%20Component%20Object%20Reference) (OtherActor :type Actor%20Object%20Reference) (OtherComp :type Primitive%20Component%20Object%20Reference) (OtherBodyIndex :type Integer) (bFromSweep :type Boolean) (SweepResult :type Hit%20Result%20Structure%20%28by%20ref%29))
  (bind _audio (Variables|Default|GetAudio))
  (if (Variables|Default|GetIsPlayerSound)
    (Audio|PushSoundMixModifier "/Game/CMP407/SoundClasses/SoundClassMixes/SC_DialogueMix.SC_DialogueMix")
    (Class|AudioComponent|SetPaused _audio false)
    (Audio|Components|Audio|SetVolumeMultiplier _audio 1.5 :!class /Script/Engine.AudioComponent)
    (Utilities|FlowControl|DoOnce false
      (:Completed
        (Audio|Components|Audio|Play _audio 0.0)))
    (else
      (Audio|PushSoundMixModifier "/Game/CMP407/SoundClasses/SoundClassMixes/SC_DialogueMix.SC_DialogueMix")
      (Audio|Components|Audio|SetVolumeMultiplier (Variables|Default|GetAudio) 1.5 :!class /Script/Engine.AudioComponent))))

(event OnComponentEndOverlap(Sphere)
  (params (OverlappedComponent :type Primitive%20Component%20Object%20Reference) (OtherActor :type Actor%20Object%20Reference) (OtherComp :type Primitive%20Component%20Object%20Reference) (OtherBodyIndex :type Integer))
  (Audio|PopSoundMixModifier "/Game/CMP407/SoundClasses/SoundClassMixes/SC_DialogueMix.SC_DialogueMix")
  (Audio|Components|Audio|SetVolumeMultiplier (Variables|Default|GetAudio) 0.2 :!class /Script/Engine.AudioComponent))

(event EventBeginPlay
  (Utilities|FlowControl|Sequence
    (:then_0
      (Variables|Default|SetPlayerReference (Game|Player|GetPlayerPawn 0))
      (Components|Sphere|SetSphereRadius (Variables|Default|GetSphere) (Variables|Default|GetSphere%20Radius) true))
    (:then_1
      (Audio|Components|Audio|SetVolumeMultiplier (Variables|Default|GetAudio) 0.2 :!class /Script/Engine.AudioComponent)
      (if (Variables|Default|GetIsPlayerSound)
        (Class|AudioComponent|SetPaused (Variables|Default|GetAudio) true)))))

(fn ConstructionScript)
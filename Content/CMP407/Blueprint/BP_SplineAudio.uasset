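; BP_SplineAudio is an actor that slides a sound along a spline to follow the player.
; On BeginPlay it caches the third-person character and starts MoveAudio, which re-calls itself on a short Delay instead of using Tick.
; Each pass moves AudioOne to the spline point closest to the player, plus X and Z offsets.
; The point is queried in Local space but applied as a world location.
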(event Custom|MoveAudio
  (bind _spline (Variables|Default|GetSpline))
  (bind _playerreference (Variables|Default|GetPlayerReference))
  (bind _returnvalue (Transformation|GetActorLocation _playerreference))
  (bind _returnvalue_2 (Spline|FindLocationClosesttoWorldLocation _spline _returnvalue "Local"))
  (Transformation|SetWorldLocation (Variables|Default|GetAudioOne) (Math|Vector|MakeVector (+ (.x _returnvalue_2) (Variables|Default|GetAudioXOffset)) (.y _returnvalue_2) (+ (.z _returnvalue_2) (Variables|Default|GetAudioZOffset))) false false)
  (Utilities|FlowControl|Delay 0.1)
  (CallFunction|MoveAudio))

(event EventBeginPlay
  (bind _asbp_third_person_character (Utilities|Casting|CastToBP_ThirdPersonCharacter (Game|GetPlayerCharacter 0)))
  (Variables|Default|SetPlayerReference _asbp_third_person_character)
  (CallFunction|MoveAudio))

(event Collision|EventActorBeginOverlap
  (params (OtherActor :type Actor%20Object%20Reference)))

(event EventTick
  (params (DeltaSeconds :type Float%20%28single-precision%29)))

(fn ConstructionScript)
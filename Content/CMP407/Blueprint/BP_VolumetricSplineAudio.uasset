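; Volumetric spline audio actor that moves an Ak (Wwise) emitter to follow the player around a spline.
; Within 500 units of the spline, the emitter sits near the pawn; otherwise it takes the closest spline point, optionally at player height.
; The emitter copies camera rotation to steady panning, and a distance-driven lazy flag swaps Tick for a looping timer.
; The construction script builds spline meshes to visualize the shape, optionally hidden in game.
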(event Custom|UpdateEmitterLocationProxy
  ;[1 1 1] Begin Play
  ;;[1 1 1] Subscribe UpdateEmitterLocation to timer by event with controllable trigger rate
  (CallFunction|UpdateEmitterSlowly))

(event Custom|Update%20Emitter%20Slowly
  (bind (_controlledpawnreference _controlledpawnlocation) (CallFunction|GetControlledPawnLocation))
  (bind (_isinsidespline_ _isinsidesplinechanged_) (CallFunction|GetIsInsideSpline))
  (bind _distancetoplayerfromclosestsplinepoint (CallFunction|GetDistancetoPlayerfromClosestSplinePoint))
  (bind _max_range_fade_distance (Variables|Default|GetMax%20Range%20Fade%20Distance))
  (bind _returnvalue (+ _max_range_fade_distance 1e+03))
  (bind _returnvalue_2 (> _distancetoplayerfromclosestsplinepoint _returnvalue))
  ;[1 1 1] Switch between tick check and no check based on lazy bool (distance)
  (if (Variables|Default|GetIs%20Lazy)
    ;[1 1 1] Find location to player and set emitter location to that location (on the spline curve)
    (Utilities|IsValid (Game|GetPlayerController 0)
      (:Is%20Valid
        (Variables|Default|SetSpline%20Curve%20Location%20Closest%20To%20Player (Spline|FindLocationClosesttoWorldLocation (Variables|Default|GetSpline) (.ControlledPawnLocation (CallFunction|GetControlledPawnLocation)) "World"))
        ;[1 1 1] Check if player is inside spline and also let us know if player went from inside to outside or vice versa. Based on that information set IsInsideSpline bool or continue without setting bool
        (if _isinsidesplinechanged_
          ;[1 1 1] Ask if dot value is more than 0 and ask the returning bool is NOT equal to the current isInside value. If it's different return true in the following branch and set isInside state to inside (dot above 0) or outside (dot below 0). Then finally ask if we are inside (true) our outside (false)
          ;;[1 1 1] Only set on state change
          (Variables|Default|SetIs%20Inside%20Spline _isinsidespline_)
          (if (not (Variables|Default|GetIs%20Initialized))
            ;;[1 1 1] Only runs false on begin play to make sure the the correct AK State inside or outside is set on begin play
            (Variables|Default|SetIs%20Initialized true :!label _label)
            (if (Variables|Default|GetIs%20Inside%20Spline) :!label _label_2
              ;[1 1 1] If inside (true) set location of emitter to tick update to player location. If outside (false) set emitter location to the closest location on the spline curve. This is used for seamless transitioning audio in and out of the spline zone. The emitter also receives the camera's rotation in order for 3d sounds to mimic the behavior of 2d sounds / reduce "stutters" and inexpedient pans when rotating the listener quickly inside the spline shape
              (Variables|Default|SetAk%20Emitter%20Location (+ (+ (Transformation|GetActorForwardVector _controlledpawnreference) "50.000000,50.000000,0.000000") _controlledpawnlocation))
              (else
                ;[1 1 1] Set emitter follow player elevation
                (if (Variables|Default|GetFollow%20Player%20Elevation)
                  (Variables|Default|SetAk%20Emitter%20Location (Math|Vector|MakeVector (.X (Math|Vector|BreakVector (Variables|Default|GetSpline%20Curve%20Location%20Closest%20To%20Player))) (.Y (Math|Vector|BreakVector (Variables|Default|GetSpline%20Curve%20Location%20Closest%20To%20Player))) (.Z (Math|Vector|BreakVector (.ControlledPawnLocation (CallFunction|GetControlledPawnLocation))))))
                  (else
                    (Variables|Default|SetAk%20Emitter%20Location (Variables|Default|GetSpline%20Curve%20Location%20Closest%20To%20Player))))))
            (Transformation|SetWorldLocationAndRotation (Variables|Default|GetAudioEmitter) (Variables|Default|GetAk%20Emitter%20Location) (CallFunction|GetPlayerControllerCameraRotation) false false)
            ;[1 1 1] Check if player is inside the spline
            (if (Variables|Default|GetIs%20Inside%20Spline)
              ;[1 1 1] To optimize performance, set lazy tick rate when more than X meters away from closest point on spline curve, else update on tick. We start ticking on tick 10 meters before entering max range to make sure RTPC starts at 1 (to make sure we get a smooth fade in)
              (if (Math|Boolean|NotEqual(Boolean) _returnvalue_2 (Variables|Default|GetIs%20Lazy))
                _
                (else
                  _))
              (Variables|Default|SetIs%20Lazy _returnvalue_2)
              ;[1 1 1] Draw debug speaker from emitter location.
              (if (Variables|Default|GetDebug)
                (Class|KismetSystemLibrary|DrawDebugConeinDegrees (Variables|Default|GetAk%20Emitter%20Location) (Math|Rotator|GetRotationXVector (CallFunction|GetPlayerControllerCameraRotation)) 1e+02 45.0 45.0 12 "(R=1.000000,G=1.000000,B=1.000000,A=1.000000)" 0.0 2.0)
                (Rendering|Debug|DrawDebugSphere (Variables|Default|GetAk%20Emitter%20Location) 1e+01 12 "(R=0.000000,G=0.344682,B=1.000000,A=1.000000)" 0.0 4.0))))
          (elif (Variables|Default|GetIs%20Initialized)
            (goto _label_2)
            (else
              (goto _label))))))
    (else
      (Actor|Tick|SetActorTickEnabled true))))

(event EventTick
  (params (DeltaSeconds :type Float%20%28single-precision%29))
  (bind (_controlledpawnreference _controlledpawnlocation) (CallFunction|GetControlledPawnLocation))
  (bind (_isinsidespline_ _isinsidesplinechanged_) (CallFunction|GetIsInsideSpline))
  (bind _distancetoplayerfromclosestsplinepoint (CallFunction|GetDistancetoPlayerfromClosestSplinePoint))
  (bind _max_range_fade_distance (Variables|Default|GetMax%20Range%20Fade%20Distance))
  (bind _returnvalue (+ _max_range_fade_distance 1e+03))
  (bind _returnvalue_2 (> _distancetoplayerfromclosestsplinepoint _returnvalue))
  ;[1 1 1] Switch between tick check and no check based on lazy bool (distance)
  (if (Variables|Default|GetIs%20Lazy)
    (Actor|Tick|SetActorTickEnabled false)
    (else
      ;[1 1 1] Find location to player and set emitter location to that location (on the spline curve)
      (Utilities|IsValid (Game|GetPlayerController 0)
        (:Is%20Valid
          (Variables|Default|SetSpline%20Curve%20Location%20Closest%20To%20Player (Spline|FindLocationClosesttoWorldLocation (Variables|Default|GetSpline) (.ControlledPawnLocation (CallFunction|GetControlledPawnLocation)) "World"))
          ;[1 1 1] Check if player is inside spline and also let us know if player went from inside to outside or vice versa. Based on that information set IsInsideSpline bool or continue without setting bool
          (if _isinsidesplinechanged_
            ;[1 1 1] Ask if dot value is more than 0 and ask the returning bool is NOT equal to the current isInside value. If it's different return true in the following branch and set isInside state to inside (dot above 0) or outside (dot below 0). Then finally ask if we are inside (true) our outside (false)
            ;;[1 1 1] Only set on state change
            (Variables|Default|SetIs%20Inside%20Spline _isinsidespline_)
            (if (not (Variables|Default|GetIs%20Initialized))
              ;;[1 1 1] Only runs false on begin play to make sure the the correct AK State inside or outside is set on begin play
              (Variables|Default|SetIs%20Initialized true :!label _label)
              (if (Variables|Default|GetIs%20Inside%20Spline) :!label _label_2
                ;[1 1 1] If inside (true) set location of emitter to tick update to player location. If outside (false) set emitter location to the closest location on the spline curve. This is used for seamless transitioning audio in and out of the spline zone. The emitter also receives the camera's rotation in order for 3d sounds to mimic the behavior of 2d sounds / reduce "stutters" and inexpedient pans when rotating the listener quickly inside the spline shape
                (Variables|Default|SetAk%20Emitter%20Location (+ (+ (Transformation|GetActorForwardVector _controlledpawnreference) "50.000000,50.000000,0.000000") _controlledpawnlocation))
                (else
                  ;[1 1 1] Set emitter follow player elevation
                  (if (Variables|Default|GetFollow%20Player%20Elevation)
                    (Variables|Default|SetAk%20Emitter%20Location (Math|Vector|MakeVector (.X (Math|Vector|BreakVector (Variables|Default|GetSpline%20Curve%20Location%20Closest%20To%20Player))) (.Y (Math|Vector|BreakVector (Variables|Default|GetSpline%20Curve%20Location%20Closest%20To%20Player))) (.Z (Math|Vector|BreakVector (.ControlledPawnLocation (CallFunction|GetControlledPawnLocation))))))
                    (else
                      (Variables|Default|SetAk%20Emitter%20Location (Variables|Default|GetSpline%20Curve%20Location%20Closest%20To%20Player))))))
              (Transformation|SetWorldLocationAndRotation (Variables|Default|GetAudioEmitter) (Variables|Default|GetAk%20Emitter%20Location) (CallFunction|GetPlayerControllerCameraRotation) false false)
              ;[1 1 1] Check if player is inside the spline
              (if (Variables|Default|GetIs%20Inside%20Spline)
                ;[1 1 1] To optimize performance, set lazy tick rate when more than X meters away from closest point on spline curve, else update on tick. We start ticking on tick 10 meters before entering max range to make sure RTPC starts at 1 (to make sure we get a smooth fade in)
                (if (Math|Boolean|NotEqual(Boolean) _returnvalue_2 (Variables|Default|GetIs%20Lazy))
                  _
                  (else
                    _))
                (Variables|Default|SetIs%20Lazy _returnvalue_2)
                ;[1 1 1] Draw debug speaker from emitter location.
                (if (Variables|Default|GetDebug)
                  (Class|KismetSystemLibrary|DrawDebugConeinDegrees (Variables|Default|GetAk%20Emitter%20Location) (Math|Rotator|GetRotationXVector (CallFunction|GetPlayerControllerCameraRotation)) 1e+02 45.0 45.0 12 "(R=1.000000,G=1.000000,B=1.000000,A=1.000000)" 0.0 2.0)
                  (Rendering|Debug|DrawDebugSphere (Variables|Default|GetAk%20Emitter%20Location) 1e+01 12 "(R=0.000000,G=0.344682,B=1.000000,A=1.000000)" 0.0 4.0))))
            (elif (Variables|Default|GetIs%20Initialized)
              (goto _label_2)
              (else
                (goto _label)))))))))

(event EventBeginPlay
  ;[1 1 1] Begin Play
  ;;[1 1 1] Subscribe UpdateEmitterLocation to timer by event with controllable trigger rate
  (Utilities|Time|SetTimerbyEvent (delegate Custom|UpdateEmitterLocationProxy) (Variables|Default|GetTimer%20Lazy) true))

(fn ConstructionScript
  (bind _spline (Variables|Default|GetSpline))
  ;[1 1 1] Run a loop to get all of our spline points and add a spline mesh for each point (used for visualizing the shape). Note: Mesh has NoCollision as we don't need it (this has been disabled for the final project)
  (for _index (range 0 (- (Spline|GetNumberOfSplinePoints (Variables|Default|GetSpline)) 1))
    (bind _returnvalue (AddComponent|AddSplineMeshComponent false)) ; Click node for details. We use a transparent material
    (SplineMesh|SetStartandEnd _returnvalue (.Location (Spline|GetLocationandTangentatSplinePoint _spline _index "Local")) (.Tangent (Spline|GetLocationandTangentatSplinePoint _spline _index "Local")) (.Location (Spline|GetLocationandTangentatSplinePoint _spline (+ _index 1) "Local")) (.Tangent (Spline|GetLocationandTangentatSplinePoint _spline (+ _index 1) "Local")) true :!class /Script/Engine.SplineMeshComponent)
    ;[1 1 1] Public bool to hide the shape in game mode
    (Development|SetHiddeninGame _returnvalue (Variables|Default|GetHidden%20In%20Game) false)))

(fn GetControlledPawnLocation
  (bind _returnvalue (Game|GetPlayerController 0))
  (bind _returnvalue_2 (Pawn|GetControlledPawn _returnvalue))
  (return _returnvalue_2 (Transformation|GetActorLocation _returnvalue_2)))

(fn GetPlayerControllerCameraRotation
  (return (Camera|GetCameraRotation (Variables|/Script/Engine.PlayerController|GetPlayerCameraManager (Game|GetPlayerController 0)))))

(fn GetIsInsideSpline
  (bind _controlledpawnlocation (CallFunction|GetControlledPawnLocation))
  (bind _spline_curve_location_closest_to_player (Variables|Default|GetSpline%20Curve%20Location%20Closest%20To%20Player))
  (bind _returnvalue (- _spline_curve_location_closest_to_player _controlledpawnlocation))
  (bind _returnvalue_2 (Math|Vector|VectorLength _returnvalue))
  (bind _returnvalue_3 (< _returnvalue_2 5e+02))
  (return _returnvalue_3 (Math|Boolean|NotEqual(Boolean) _returnvalue_3 (Variables|Default|GetIs%20Inside%20Spline))))

(fn GetDistancetoPlayerfromClosestSplinePoint
  ;[1 1 1] Substract the location of our audio emitter from the player's location to get the distance between the closest point on the spline curve and the player
  (return (Math|Vector|VectorLength (- (Variables|Default|GetAk%20Emitter%20Location) (Transformation|GetActorLocation (Pawn|GetControlledPawn (Game|GetPlayerController 0)))))))
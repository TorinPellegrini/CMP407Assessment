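; Volumetric Wwise emitter actor that plays an Ak event from the static mesh collision point nearest the player.
; It offsets that point slightly, matches camera rotation, and switches from Tick to a looping lazy timer beyond fade range plus a margin.
; Character overlaps set inside/outside Wwise states.
; The fade-distance RTPC starts at zero; its distance-mapped update sits behind an always-false branch, though debug output still prints that value.
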(event Custom|UpdateEmitterLocationProxy
  ;[1 1 1] Begin Play
  ;;[1 1 1] Subscribe UpdateEmitterLocation to timer by event with controllable trigger rate
  (CallFunction|UpdateEmitterSlowly))

(event Custom|Update%20Emitter%20Slowly
  (bind (_controlledpawnreference _controlledpawnlocation) (CallFunction|GetControlledPawnLocation))
  (bind _distancetoplayerfromclosestsplinepoint (CallFunction|GetDistancetoPlayerfromClosestPointonMesh))
  (bind _distancetoplayerfromclosestsplinepoint_2 (CallFunction|GetDistancetoPlayerfromClosestPointonMesh))
  (bind _max_range_fade_distance (Variables|Default|GetMax%20Range%20Fade%20Distance))
  (bind _max_range_fade_distance_2 (Variables|Default|GetMax%20Range%20Fade%20Distance))
  (bind _returnvalue (Math|Float|MapRangeClamped _distancetoplayerfromclosestsplinepoint _max_range_fade_distance 0.0 1.0 0.0))
  (bind _returnvalue_2 (+ _max_range_fade_distance_2 1e+03))
  (bind _returnvalue_3 (> _distancetoplayerfromclosestsplinepoint_2 _returnvalue_2))
  ;[1 1 1] Switch between tick check and no check based on lazy bool (distance)
  (if (Variables|Default|GetIs%20Lazy)
    ;[1 1 1] Find the location on the static mesh that is closest to the player and move it slightly forward to create a more varying stero image when the player rotates within the static mesh
    (Utilities|IsValid (Game|GetPlayerController 0)
      (:Is%20Valid
        (bind _output_get (Variables|Default|SetStatic%20Mesh%20Location%20Closest%20To%20Player (+ (.OutPointOnBody (Collision|GetClosestPointonCollision (Variables|Default|GetStaticMesh) _controlledpawnlocation "None")) (+ (Transformation|GetActorForwardVector _controlledpawnreference) "0.000000,75.000000,0.000000"))))
        ;[1 1 1] Set the Ak Emitter's location and make it follow the camera's rotation
        (Transformation|SetWorldLocationAndRotation (Variables|Default|GetAkComponent) _output_get (CallFunction|GetPlayerControllerCameraRotation) false false)
        ;[1 1 1] Set RTPC for fade distance to make (especially 2d) sounds fade out when moving out away from the static mesh or moving towards it. Don't set when inside static mesh
        (if true
          _
          (else
            (CallFunction|SetRTPCValue (Variables|Default|GetAkComponent) "rtpc_area_fade_distance" _returnvalue)))
        ;[1 1 1] To optimize performance, set lazy tick rate when more than X meters away from closest point on static mesh, else update on tick. We start ticking on tick 10 meters before entering max range to make sure RTPC starts at 1 (to make sure we get a smooth fade in)
        (if (Math|Boolean|NotEqual(Boolean) _returnvalue_3 (Variables|Default|GetIs%20Lazy))
          _
          (else
            _))
        (Variables|Default|SetIs%20Lazy _returnvalue_3)
        ;[1 1 1] Draw debug speaker from emitter location as well as RTPC value and if we're currently inside or outside emitter
        (if (Variables|Default|GetDebug)
          (Class|KismetSystemLibrary|DrawDebugConeinDegrees (Variables|Default|GetStatic%20Mesh%20Location%20Closest%20To%20Player) (Math|Rotator|GetRotationXVector (CallFunction|GetPlayerControllerCameraRotation)) 1e+02 45.0 45.0 12 "(R=1.000000,G=1.000000,B=1.000000,A=1.000000)" 0.0 2.0)
          (Rendering|Debug|DrawDebugSphere (Variables|Default|GetStatic%20Mesh%20Location%20Closest%20To%20Player) 1e+01 12 "(R=0.000000,G=0.344682,B=1.000000,A=1.000000)" 0.0 4.0)
          (if (Variables|Default|GetIs%20Lazy)
            _
            (else
              (Utilities|FlowControl|Delay 0.2)))
          (Development|PrintString (Utilities|String|ToString(Text) (Utilities|Text|FormatText "Debug SPE - RTPC:{RTPC}  |  Lazy?: {Lazy}  |  Is Inside?: {IsInside}" (Utilities|Text|ToText(Float) _returnvalue "HalfToEven" false true 2 2 0 2) (Utilities|Text|ToText(Boolean) (Variables|Default|GetIs%20Lazy)) (Utilities|Text|ToText(Boolean) (Variables|Default|GetIs%20Inside%20Static%20Mesh))))))))
    (else
      (Actor|Tick|SetActorTickEnabled true))))

(event Collision|EventActorEndOverlap
  (params (OtherActor :type Actor%20Object%20Reference))
  ;[0.1036 0.4193 1] Set AK state based on inside or outside
  (Utilities|Casting|CastToCharacter OtherActor)
  (Class|AnimationStateMachineLibrary|SetState :BlendType "TLT_StandardBlend" :AlphaBlendOption "Linear" :StateGroup (Variables|Default|GetState%20Group) :State (Variables|Default|GetState%20Outside))
  (Variables|Default|SetIs%20Inside%20Static%20Mesh false))

(event EventTick
  (params (DeltaSeconds :type Float%20%28single-precision%29))
  (bind (_controlledpawnreference _controlledpawnlocation) (CallFunction|GetControlledPawnLocation))
  (bind _distancetoplayerfromclosestsplinepoint (CallFunction|GetDistancetoPlayerfromClosestPointonMesh))
  (bind _distancetoplayerfromclosestsplinepoint_2 (CallFunction|GetDistancetoPlayerfromClosestPointonMesh))
  (bind _max_range_fade_distance (Variables|Default|GetMax%20Range%20Fade%20Distance))
  (bind _max_range_fade_distance_2 (Variables|Default|GetMax%20Range%20Fade%20Distance))
  (bind _returnvalue (Math|Float|MapRangeClamped _distancetoplayerfromclosestsplinepoint _max_range_fade_distance 0.0 1.0 0.0))
  (bind _returnvalue_2 (+ _max_range_fade_distance_2 1e+03))
  (bind _returnvalue_3 (> _distancetoplayerfromclosestsplinepoint_2 _returnvalue_2))
  ;[1 1 1] Switch between tick check and no check based on lazy bool (distance)
  (if (Variables|Default|GetIs%20Lazy)
    (Actor|Tick|SetActorTickEnabled false)
    (else
      ;[1 1 1] Find the location on the static mesh that is closest to the player and move it slightly forward to create a more varying stero image when the player rotates within the static mesh
      (Utilities|IsValid (Game|GetPlayerController 0)
        (:Is%20Valid
          (bind _output_get (Variables|Default|SetStatic%20Mesh%20Location%20Closest%20To%20Player (+ (.OutPointOnBody (Collision|GetClosestPointonCollision (Variables|Default|GetStaticMesh) _controlledpawnlocation "None")) (+ (Transformation|GetActorForwardVector _controlledpawnreference) "0.000000,75.000000,0.000000"))))
          ;[1 1 1] Set the Ak Emitter's location and make it follow the camera's rotation
          (Transformation|SetWorldLocationAndRotation (Variables|Default|GetAkComponent) _output_get (CallFunction|GetPlayerControllerCameraRotation) false false)
          ;[1 1 1] Set RTPC for fade distance to make (especially 2d) sounds fade out when moving out away from the static mesh or moving towards it. Don't set when inside static mesh
          (if true
            _
            (else
              (CallFunction|SetRTPCValue (Variables|Default|GetAkComponent) "rtpc_area_fade_distance" _returnvalue)))
          ;[1 1 1] To optimize performance, set lazy tick rate when more than X meters away from closest point on static mesh, else update on tick. We start ticking on tick 10 meters before entering max range to make sure RTPC starts at 1 (to make sure we get a smooth fade in)
          (if (Math|Boolean|NotEqual(Boolean) _returnvalue_3 (Variables|Default|GetIs%20Lazy))
            _
            (else
              _))
          (Variables|Default|SetIs%20Lazy _returnvalue_3)
          ;[1 1 1] Draw debug speaker from emitter location as well as RTPC value and if we're currently inside or outside emitter
          (if (Variables|Default|GetDebug)
            (Class|KismetSystemLibrary|DrawDebugConeinDegrees (Variables|Default|GetStatic%20Mesh%20Location%20Closest%20To%20Player) (Math|Rotator|GetRotationXVector (CallFunction|GetPlayerControllerCameraRotation)) 1e+02 45.0 45.0 12 "(R=1.000000,G=1.000000,B=1.000000,A=1.000000)" 0.0 2.0)
            (Rendering|Debug|DrawDebugSphere (Variables|Default|GetStatic%20Mesh%20Location%20Closest%20To%20Player) 1e+01 12 "(R=0.000000,G=0.344682,B=1.000000,A=1.000000)" 0.0 4.0)
            (if (Variables|Default|GetIs%20Lazy)
              _
              (else
                (Utilities|FlowControl|Delay 0.2)))
            (Development|PrintString (Utilities|String|ToString(Text) (Utilities|Text|FormatText "Debug SPE - RTPC:{RTPC}  |  Lazy?: {Lazy}  |  Is Inside?: {IsInside}" (Utilities|Text|ToText(Float) _returnvalue "HalfToEven" false true 2 2 0 2) (Utilities|Text|ToText(Boolean) (Variables|Default|GetIs%20Lazy)) (Utilities|Text|ToText(Boolean) (Variables|Default|GetIs%20Inside%20Static%20Mesh)))))))))))

(event Collision|EventActorBeginOverlap
  (params (OtherActor :type Actor%20Object%20Reference))
  ;[0.1036 0.4193 1] Set AK state based on inside or outside
  (Utilities|Casting|CastToCharacter OtherActor)
  (Class|AnimationStateMachineLibrary|SetState :BlendType "TLT_StandardBlend" :AlphaBlendOption "Linear" :StateGroup (Variables|Default|GetState%20Group) :State (Variables|Default|GetState%20Inside))
  (Variables|Default|SetIs%20Inside%20Static%20Mesh true))

(event EventBeginPlay
  ;[1 1 1] Begin Play
  ;;[0.1036 0.4193 1] Trigger AK Event on begin play
  (Utilities|FlowControl|Sequence
    (:then_0
      (CallFunction|PostAkEvent (Variables|Default|GetAkComponent) (.Ak%20Event%20Emitter (Variables|Default|GetAk%20Event%20Emitter)))
      ;;[1 1 1] Set initial RTPC to ensure it's being set when spawning inside of zone
      (CallFunction|SetRTPCValue (Variables|Default|GetAkComponent) "rtpc_area_fade_distance" 0.0))
    (:then_1
      ;;[1 1 1] Subscribe UpdateEmitterLocation to timer by event with controllable trigger rate
      (Utilities|Time|SetTimerbyEvent (delegate Custom|UpdateEmitterLocationProxy) (Variables|Default|GetTimer%20Lazy) true))))

(fn ConstructionScript
  ;[1 1 1] Puplic occlusion refresh interval
  (Variables|Default|SetOcclusionRefreshInterval (Variables|Default|GetAkComponent) (Variables|Default|GetOcc%20Refresh%20Interval))
  (Components|StaticMesh|SetStaticMesh (Variables|Default|GetStaticMesh) (Variables|Default|GetMesh))
  (Development|SetHiddeninGame (Variables|Default|GetDefaultSceneRoot) (Variables|Default|GetHidden%20In%20Game) true)
  (Rendering|SetVisibility (Variables|Default|GetDefaultSceneRoot) (Variables|Default|GetVisibleInEditor) true))

(fn GetControlledPawnLocation
  (bind _returnvalue (Game|GetPlayerController 0))
  (bind _returnvalue_2 (Pawn|GetControlledPawn _returnvalue))
  (return _returnvalue_2 (Transformation|GetActorLocation _returnvalue_2)))

(fn GetPlayerControllerCameraRotation
  (return (Camera|GetCameraRotation (Variables|/Script/Engine.PlayerController|GetPlayerCameraManager (Game|GetPlayerController 0)))))

(fn GetDistancetoPlayerfromClosestPointonMesh
  ;[1 1 1] Substract the location of our audio emitter from the player's location to get the distance between the closest point in the static mesh and the player
  (return (Math|Vector|VectorLength (- (Variables|Default|GetStatic%20Mesh%20Location%20Closest%20To%20Player) (Transformation|GetActorLocation (Pawn|GetControlledPawn (Game|GetPlayerController 0)))))))